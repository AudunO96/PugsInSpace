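; PugPlayer_BP is the player Blueprint for the pug, handling HUD creation and pausing.
; BeginPlay creates the HUD widget, stores a reference and adds it to the viewport.
; Pressing P lazily creates and reuses the PauseMenu widget, switches input to UI-only focused on it, displays it and pauses the game.
; The Blueprint contains no movement or unpause logic, and its construction script is empty.
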(event EventBeginPlay
  (bind _returnvalue (UserInterface|CreateWidget "/Game/HUD.HUD_C"))
  (bind _output_get (Variables|Default|SetHUD%20Reference _returnvalue))
  (UserInterface|Viewport|AddtoViewport _output_get 0))

(event Collision|EventActorBeginOverlap
  (params (OtherActor :type Actor%20Object%20Reference)))

(event EventTick
  (params (DeltaSeconds :type Float%20%28single-precision%29)))

(event Input|KeyboardEvents|P
  (params (Key :type Key%20Structure :default "AnyKey"))
  (:Pressed
    (Utilities|IsValid (Variables|Default|GetPauseMenu%20Reference)
      (:Is%20Valid
        _)
      (:Is%20Not%20Valid
        (bind _returnvalue (UserInterface|CreateWidget "/Game/PauseMenu.PauseMenu_C"))
        (Variables|Default|SetPauseMenu%20Reference _returnvalue)))
    (Input|SetInputModeUIOnly (Game|GetPlayerController 0) (Variables|Default|GetPauseMenu%20Reference) "DoNotLock")
    (UserInterface|Viewport|AddtoViewport (Variables|Default|GetPauseMenu%20Reference) 0)
    (Game|SetGamePaused true)))

(fn ConstructionScript)